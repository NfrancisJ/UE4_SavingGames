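; Player pawn Blueprint with axis-driven movement and look, plus debug keys to print coins, save and load.
; Save and load run through BP_GameInstance event dispatchers, bound on BeginPlay and fired by key presses.
; On save, it writes the pawn transform into the shared save object while keeping the coin count.
; The load handler is empty; transform restore, slot saving and restart logic remain disconnected.
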(event `InputAxis|Move`
  (params (AxisValue :type "Float (single-precision)"))
  (`self.AddMovementInput` (`KismetMathLibrary.GetForwardVector` (`self.GetControlRotation`)) AxisValue))

(event `InputAxis|Straf`
  (params (AxisValue :type "Float (single-precision)"))
  (`self.AddMovementInput` (`KismetMathLibrary.GetRightVector` (`self.GetControlRotation`)) AxisValue))

(event `InputAxis|Look-Y`
  (params (AxisValue :type "Float (single-precision)"))
  (`self.AddControllerPitchInput` AxisValue))

(event `InputAxis|Look-X`
  (params (AxisValue :type "Float (single-precision)"))
  (`self.AddControllerYawInput` AxisValue))

(event `self.ReceiveBeginPlay`
  (bind _asbp_game_instance (cast `/Game/MyGame/Blueprints/Core/BP_GameInstance` (`GameplayStatics.GetGameInstance`)))
  (bind _output_get (set `self.GameInstance` _asbp_game_instance))
  (add `/Game/MyGame/Blueprints/Core/BP_GameInstance.OnSave` _output_get (delegate `OnSave`))
  ;[1 0 0] temp disconnect
  (add `/Game/MyGame/Blueprints/Core/BP_GameInstance.OnLoad` _output_get (delegate `OnLoad_Event_0`)))

(event `OnSave`
  (bind _savegameobject (`/Game/MyGame/Blueprints/Core/BP_GameInstance.SaveGameObject` (`self.GameInstance`)))
  (bind (_splayer_transform _splayer_coins) (break `/Game/MyGame/Blueprints/Core/Structs/SPlayer` (`/Game/MyGame/Blueprints/Core/BP_SaveGame.SPlayer` _savegameobject)))
  (set `/Game/MyGame/Blueprints/Core/BP_SaveGame.SPlayer` (make `/Game/MyGame/Blueprints/Core/Structs/SPlayer` (`self.GetTransform` (`GameplayStatics.GetPlayerPawn` 0)) _splayer_coins) _savegameobject))

(event `OnLoad_Event_0`
  ;[1 0 0] temp disconnect
)

(event `Key|P`
  (params (Key :type "Key Structure"))
  (bind (_splayer_transform _splayer_coins) (break `/Game/MyGame/Blueprints/Core/Structs/SPlayer` (`/Game/MyGame/Blueprints/Core/BP_SaveGame.SPlayer` (`/Game/MyGame/Blueprints/Core/BP_GameInstance.SaveGameObject` (`self.GameInstance`)))))
  (:`Pressed`
    (`KismetSystemLibrary.PrintString` (`KismetStringLibrary.Conv_IntToString` _splayer_coins))))

(event `Key|E`
  (params (Key :type "Key Structure"))
  (:`Pressed`
    (`/Game/MyGame/Blueprints/Core/BP_GameInstance.OnSave` (`self.GameInstance`))))

(event `Key|R`
  (params (Key :type "Key Structure"))
  (:`Pressed`
    (`/Game/MyGame/Blueprints/Core/BP_GameInstance.OnLoad` (`self.GameInstance`))))

(fn `UserConstructionScript`)