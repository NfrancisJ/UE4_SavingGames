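; BP_Light is an interactable light whose point light toggles visibility when the player character begins overlapping it, after running the parent overlap logic.
; Save writes the light's visibility to the SLight map in the GameInstance's save object, keyed by object name, removing the entry when the light is hidden.
; Load applies the looked-up value, so only visible lights need storing, with hidden treated as the default.
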(event `self.ReceiveActorBeginOverlap`
  (params (OtherActor :type "Actor Object Reference"))
  (`parent.ReceiveActorBeginOverlap` OtherActor)
  (if (== OtherActor (`GameplayStatics.GetPlayerCharacter` 0))
    (`SceneComponent.ToggleVisibility` (`self.PointLight`) false)))

(event `self.Save`
  (bind _returnvalue (`KismetSystemLibrary.GetObjectName` self))
  (bind _slight (`/Game/MyGame/Blueprints/Core/BP_SaveGame.SLight` (`/Game/MyGame/Blueprints/Core/BP_GameInstance.SaveGameObject` (`self.GameInstance`))))
  ;[0 0 0] Check to see if the light equals the default value. If it is, Remove it from the MAP, else Add it to the MAP.
  (if (== false (`SceneComponent.bVisible` (`self.PointLight`)))
    (`BlueprintMapLibrary.Map_Remove` _slight _returnvalue)
    (else
      (`BlueprintMapLibrary.Map_Add` _slight _returnvalue (make `/Game/MyGame/Blueprints/Core/Structs/SLight` (`SceneComponent.bVisible` (`self.PointLight`)))))))

(event `self.Load`
  ;[0 0 0] Fetch Light values from the Savegame and set it.
  (`SceneComponent.SetVisibility` (`self.PointLight`) (break `/Game/MyGame/Blueprints/Core/Structs/SLight` (`BlueprintMapLibrary.Map_Find` (`/Game/MyGame/Blueprints/Core/BP_SaveGame.SLight` (`/Game/MyGame/Blueprints/Core/BP_GameInstance.SaveGameObject` (`self.GameInstance`))) (`KismetSystemLibrary.GetObjectName` self))) false))

(fn `UserConstructionScript`)